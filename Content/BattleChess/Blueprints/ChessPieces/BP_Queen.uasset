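; BP_Queen is the queen chess piece Blueprint in BattleChess, defining which squares the queen can move to.
; ShowPossibleMoves clears existing highlights through the game mode reference, then highlights diagonal, horizontal and vertical squares using the piece's Color.
; The function returns the IsKing flag, and the construction script only calls its parent.
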(fn `ShowPossibleMoves`
  (returns (IsKing :type Boolean))
  (locals (TempEvalLegality :type Boolean) (price :type Integer))
  (`|ExecutionSequence`
    (:`then_0`
      (`/Game/BattleChess/Blueprints/BP_GameMode.UnhighlightSquares` (`self.GameModeRef`)))
    (:`then_1`
      (`self.HighlightDiagonalSquares` (`self.Color`)))
    (:`then_2`
      (`self.HighlightHorizontal Squares` (`self.Color`)))
    (:`then_3`
      (`self.HighlightVerticalSquares` (`self.Color`)))
    (:`then_4`
      (return (`self.IsKing`)))))

(fn `UserConstructionScript`
  (`parent.UserConstructionScript`))