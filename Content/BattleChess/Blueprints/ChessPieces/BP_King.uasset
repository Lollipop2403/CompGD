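; King chess piece for Battle Chess that highlights the squares it can move or castle to.
; ShowPossibleMoves clears old highlights, then marks each adjacent square that is on the board and free of friendly pieces, without testing for check.
; If the king is unmoved, uncastled and not in check, EvaluateCastlePath scans both ways along Y for an unblocked, unmoved rook and highlights the square two steps toward it.
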(fn `EvaluateCastlePath`
  (params (YInc :type Integer))
  (locals (CanContinue :type Boolean) (IsPositive :type Boolean) (TempY :type Integer))
  (bind (_occupant _isoccupied) (`/Game/BattleChess/Blueprints/BP_GameMode.GetOccupant` (`self.GameModeRef`) (`self.X`) (`local.TempY`) (`self.Color`)))
  (bind (_asbp_rook _bsuccess) (cast `/Game/BattleChess/Blueprints/ChessPieces/BP_Rook` _occupant :!pure true))
  (set `local.IsPositive` (> YInc 0))
  (set `local.TempY` (`self.Y`))
  (set `local.CanContinue` true)
  (while (`local.CanContinue`)
    (set `local.TempY` (+ YInc (`local.TempY`)))
    (if (and (< (`local.TempY`) 8) (> (`local.TempY`) 1))
      (set `local.CanContinue` (not (`.IsOccupied` (`/Game/BattleChess/Blueprints/BP_GameMode.GetOccupant` (`self.GameModeRef`) (`self.X`) (`local.TempY`) (`self.Color`))))) ; If not occupied, continue evaluating squares...
      (else
        (if (and _bsuccess _isoccupied)
          (if (`/Game/BattleChess/Blueprints/ChessPieces/BP_ChessPiece.IsInitialMove` _asbp_rook)
            (`self.HighlightCastleSquares` (`local.IsPositive`)) ; Highlight square as potential move...
          ))
        (set `local.CanContinue` false)))))

(fn `EvaluateCastleSquares`
  (locals (RookA :type "/Game/BattleChess/Blueprints/ChessPieces/BP_ChessPiece Object Reference") (RookB :type "/Game/BattleChess/Blueprints/ChessPieces/BP_ChessPiece Object Reference") (TempX :type Integer) (TempY :type Integer) (CanContinue :type Boolean))
  (set `self.KindCanCastle` false)
  (if (not (`self.KingHasCastled`))
    (if (`self.IsInitialMove`)
      (if (not (`/Game/BattleChess/Blueprints/BP_GameMode.Is Active King Check Status` (`self.GameModeRef`)))
        (`|ExecutionSequence`
          (:`then_0`
            (`self.EvaluateCastlePath` 1))
          (:`then_1`
            (`self.EvaluateCastlePath` -1)))
        (else
          (set `self.KindCanCastle` false :!label _label)))
      (else
        (goto _label)))))

(fn `HighlightCastleSquares`
  (params (IsPositive :type Boolean))
  (locals (TempY :type Integer))
  (if IsPositive
    (bind _output_get (set `local.TempY` (+ (`self.Y`) 2)))
    (`self.HighlightPotentialSquare` (`self.X`) _output_get (`self.Color`))
    (set `self.KindCanCastle` true)
    (else
      (bind _output_get_2 (set `local.TempY` (+ (`self.Y`) -2)))
      (`self.HighlightPotentialSquare` (`self.X`) _output_get_2 (`self.Color`))
      (set `self.KindCanCastle` true))))

(fn `HighlightKingSquare`
  (params (XIncr :type Integer) (YIncr :type Integer))
  (locals (TempX :type Integer) (TempY :type Integer))
  (set `local.TempX` (+ (`self.X`) XIncr))
  (set `local.TempY` (+ (`self.Y`) YIncr))
  (if (`self.IsValidMoveForKing` (`local.TempX`) (`local.TempY`))
    (`self.HighlightPotentialSquare` (`local.TempX`) (`local.TempY`) (`self.Color`) false (`/Game/BattleChess/Blueprints/BP_PlayerController.bought` (`self.PlayerControllerRef`)))))

(fn `IsValidMoveForKing`
  (params (X :type Integer) (Y :type Integer))
  (returns (IsValidMove :type Boolean))
  (bind (_occupant _isoccupied _isoccupiedbyfriend _isvalidsquare) (`/Game/BattleChess/Blueprints/BP_GameMode.GetOccupant` (`self.GameModeRef`) X Y (`self.Color`)))
  (if _isvalidsquare
    (if _isoccupiedbyfriend
      (return false) ; FALSE: Occupied by friend
      (else
        (return true) ; TRUE: Empty or has opponent
      ))
    (else
      (return false) ; FALSE: Invalid square
    )))

(fn `ShowPossibleMoves`
  (returns (IsKing :type Boolean))
  (`|ExecutionSequence`
    (:`then_0`
      (`/Game/BattleChess/Blueprints/BP_GameMode.UnhighlightSquares` (`self.GameModeRef`))
      (set `self.KindCanCastle` false)
      (set `self.KingIsCastling` false))
    (:`then_1`
      (`self.HighlightKingSquare` 1)
      (`self.HighlightKingSquare` 1 1)
      (`self.HighlightKingSquare` 1 -1))
    (:`then_2`
      (`self.HighlightKingSquare` -1)
      (`self.HighlightKingSquare` -1 1)
      (`self.HighlightKingSquare` -1 -1))
    (:`then_3`
      (`self.HighlightKingSquare` 0 1)
      (`self.HighlightKingSquare` 0 -1))
    (:`then_4`
      (`self.EvaluateCastleSquares`)
      (return (`self.IsKing`)))))

(fn `ShowPossibleMoves_0_0`
  (returns (IsKing :type Boolean))
  (locals (price :type Integer))
  (`|ExecutionSequence`
    (:`then_0`
      (`/Game/BattleChess/Blueprints/BP_GameMode.UnhighlightSquares` (`self.GameModeRef`))
      (set `self.KindCanCastle` false)
      (set `self.KingIsCastling` false))
    (:`then_1`
      (`self.HighlightKingSquare` 1)
      (`self.HighlightKingSquare` 1 1)
      (`self.HighlightKingSquare` 1 -1))
    (:`then_2`
      (`self.HighlightKingSquare` -1)
      (`self.HighlightKingSquare` -1 1)
      (`self.HighlightKingSquare` -1 -1))
    (:`then_3`
      (`self.HighlightKingSquare` 0 1)
      (`self.HighlightKingSquare` 0 -1))
    (:`then_4`
      (`self.EvaluateCastleSquares`)
      (return (`self.IsKing`)))))

(fn `UserConstructionScript`
  (`parent.UserConstructionScript`))