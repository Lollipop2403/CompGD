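; BP_Bishop is the bishop chess piece in BattleChess, a child Blueprint that defines the piece's move highlighting.
; ShowPossibleMoves clears existing square highlights through the game mode, then highlights diagonal squares for the piece's color, passing the player controller's Bought flag as the placement-move indicator.
; It returns the piece's IsKing flag, and the construction script only calls the parent.
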(fn `ShowPossibleMoves`
  (returns (IsKing :type Boolean))
  (`|ExecutionSequence`
    (:`then_0`
      (`/Game/BattleChess/Blueprints/BP_GameMode.UnhighlightSquares` (`self.GameModeRef`)))
    (:`then_1`
      (`self.HighlightDiagonalSquares` (`self.Color`) (`/Game/BattleChess/Blueprints/BP_PlayerController.bought` (`self.PlayerControllerRef`))))
    (:`then_2`
      (return (`self.IsKing`)))))

(fn `UserConstructionScript`
  (`parent.UserConstructionScript`))