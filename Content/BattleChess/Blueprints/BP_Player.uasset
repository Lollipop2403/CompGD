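; BattleChess player Blueprint that holds both players' state, moves the camera between White and Black views, and toggles the pause menu.
; Setters rebuild the whole player struct to change one field, covering color, name, check, moves, captures and Chesscoins.
; Purchases check the active player's coins from BP_GameMode and a figure cap, then deduct the price and count the figure.
; Bought figures are only printed, and debug keys test the economy.
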(event Custom|SetPlayerCamera
  (params (PlayerColor :type EN_PlayerColor%20Enum :default "NewEnumerator0"))
  (bind _white (Variables|Default|GetWhite))
  (bind _black (Variables|Default|GetBlack))
  (bind _returnvalue (Transformation|GetRelativeTransform _black))
  (bind _returnvalue_2 (Transformation|GetRelativeTransform _white))
  (Components|MoveComponentTo (Variables|Default|GetCameraAzimuth) "0, 0, 0" "0, 0, 0" true true 1.0 true)
  (switch Utilities|FlowControl|Switch|SwitchonEN_PlayerColor PlayerColor
    (:NewEnumerator0
      (Components|MoveComponentTo (Variables|Default|GetCamera) (.location _returnvalue_2) (.rotation _returnvalue_2) true true 3.0 false))
    (:NewEnumerator1
      (Components|MoveComponentTo (Variables|Default|GetCamera) (.location _returnvalue) (.rotation _returnvalue) true true 3.0 false))))

(event Custom|Remove%20Chesscoin
  (params (BoughtFigure :type BP%20Chess%20Piece%20Class%20Reference))
  (bind _pricechesscoin (Utilities|GetClassDefaults BoughtFigure))
  ;[1 0.6953 0] Currency Chesscoin System
  (if (Utilities|IsValidClass BoughtFigure)
    (bind _asbp_game_mode (Utilities|Casting|CastToBP_GameMode (Game|GetGameMode)))
    (if (>= (.currentChesscoins (Utilities|Struct|BreakST_Player (Default|GetActivePlayer _asbp_game_mode))) _pricechesscoin)
      (if (< (.BoughtFigures (Utilities|Struct|BreakST_Player (Default|GetActivePlayer _asbp_game_mode))) (Variables|Default|GetmaxBoughtFigures))
        (GamePlay|SetPlayerChesscoins (.Index (Utilities|Struct|BreakST_Player (Default|GetActivePlayer _asbp_game_mode))) (- (.currentChesscoins (Utilities|Struct|BreakST_Player (Default|GetActivePlayer _asbp_game_mode))) _pricechesscoin))
        (CallFunction|GetChessFigure BoughtFigure)
        (GamePlay|SetBoughtFigures (.Index (Utilities|Struct|BreakST_Player (Default|GetActivePlayer _asbp_game_mode))))
        (else
          (bind _output_get (Variables|Default|SetinsufficientFundsMessage "Du hast die maximale Anzahl an Spielfiguren gekauft"))
          (Development|PrintText _output_get)))
      (else
        (bind _output_get_2 (Variables|Default|SetinsufficientFundsMessage "Du hast nicht genug Chess Coins um dir das zu kaufen."))
        (Development|PrintText _output_get_2)))))

(event Custom|Add%20Chesscoin
  (params (addedChesscoin :type Integer))
  ;[1 0.6953 0] Currency Chesscoin System
  (bind _asbp_game_mode (Utilities|Casting|CastToBP_GameMode (Game|GetGameMode)))
  (GamePlay|SetPlayerChesscoins (.Index (Utilities|Struct|BreakST_Player (Default|GetActivePlayer _asbp_game_mode))) (+ (.currentChesscoins (Utilities|Struct|BreakST_Player (Default|GetActivePlayer _asbp_game_mode))) addedChesscoin)))

(event Custom|Get%20ChessFigure
  (params (BoughtFigure :type BP%20Chess%20Piece%20Class%20Reference))
  ;[1 1 1] Chess Figure System
  (Development|PrintString "Schachfigur gekauft:")
  (Development|PrintString (Utilities|GetClassDisplayName BoughtFigure) true true "(R=0.536458,G=0.007120,B=0.103760,A=1.000000)"))

(event Input|ActionEvents|InputActionPauseGame
  (params (Key :type Key%20Structure :default "None"))
  (bind _returnvalue (Game|GetPlayerController 0))
  ;[1 1 1] Pause Menu
  (:Pressed
    (Utilities|IsValid (Variables|Default|GetPauseMenuREF)
      (:Is%20Valid
        _)
      (:Is%20Not%20Valid
        (bind _returnvalue_2 (UserInterface|CreateWidget "/Game/BattleChess/UI/Pause_Menu/Pause_M.Pause_M_C"))
        (Variables|Default|SetPauseMenuREF _returnvalue_2)))
    (if (Game|IsGamePaused)
      (Widget|RemovefromParent (Variables|Default|GetPauseMenuREF))
      (Game|SetGamePaused false)
      (Variables|/Script/Engine.PlayerController|SetbShowMouseCursor _returnvalue false)
      (else
        (UserInterface|Viewport|AddtoViewport (Variables|Default|GetPauseMenuREF) 0)
        (Game|SetGamePaused true)
        (Variables|/Script/Engine.PlayerController|SetbShowMouseCursor _returnvalue false)
        (Input|SetInputModeGameandUI 0 (Variables|Default|GetPauseMenuREF) "LockInFullscreen" false false)))))

(event Input|KeyboardEvents|DebugKey1
  (params (Key :type Key%20Structure :default "None") (ActionValue :type Input%20Action%20Value%20Structure))
  ;[1 0.9452 0.243] Debug Currency Chesscoin
  (:Pressed
    (CallFunction|AddChesscoin 30)))

(event Input|KeyboardEvents|DebugKey2
  (params (Key :type Key%20Structure :default "None") (ActionValue :type Input%20Action%20Value%20Structure))
  ;[1 0.9452 0.243] Debug Currency Chesscoin
  (:Pressed
    (CallFunction|RemoveChesscoin "/Game/BattleChess/Blueprints/ChessPieces/BP_Knight.BP_Knight_C")))

(fn ConstructionScript)

(fn GetPlayerbyIndex
  (params (PlayerIndex :type Integer))
  (if (== PlayerIndex (.index (Variables|Default|GetPlayer0)))
    (return (Variables|Default|GetPlayer0))
    (else
      (return (Variables|Default|GetPlayer1)))))

(fn GetPlayerbyColor
  (params (PlayerColor :type EN_PlayerColor%20Enum :default "NewEnumerator0"))
  (if (Utilities|Enum|Equal(Enum) PlayerColor (.color (Variables|Default|GetPlayer0)))
    (return (Variables|Default|GetPlayer0))
    (else
      (return (Variables|Default|GetPlayer1)))))

(fn SetPlayerColor
  (params (PlayerIndex :type Integer) (PlayerColor :type EN_PlayerColor%20Enum :default "NewEnumerator0"))
  (switch int PlayerIndex
    (:0
      (Variables|Default|SetPlayer0 (Utilities|Struct|MakeST_Player (.Name (Utilities|Struct|BreakST_Player (Variables|Default|GetPlayer0))) PlayerColor (.Index (Utilities|Struct|BreakST_Player (Variables|Default|GetPlayer0))) (.isInCheckFlag (Utilities|Struct|BreakST_Player (Variables|Default|GetPlayer0))) (.HasLegalMoves (Utilities|Struct|BreakST_Player (Variables|Default|GetPlayer0))) (.MoveCount (Utilities|Struct|BreakST_Player (Variables|Default|GetPlayer0))) (.Captures (Utilities|Struct|BreakST_Player (Variables|Default|GetPlayer0))) (.currentChesscoins (Utilities|Struct|BreakST_Player (Variables|Default|GetPlayer0))))))
    (:1
      (Variables|Default|SetPlayer1 (Utilities|Struct|MakeST_Player (.Name (Utilities|Struct|BreakST_Player (Variables|Default|GetPlayer1))) PlayerColor (.Index (Utilities|Struct|BreakST_Player (Variables|Default|GetPlayer1))) (.isInCheckFlag (Utilities|Struct|BreakST_Player (Variables|Default|GetPlayer1))) (.HasLegalMoves (Utilities|Struct|BreakST_Player (Variables|Default|GetPlayer1))) (.MoveCount (Utilities|Struct|BreakST_Player (Variables|Default|GetPlayer1))) (.Captures (Utilities|Struct|BreakST_Player (Variables|Default|GetPlayer1))) (.currentChesscoins (Utilities|Struct|BreakST_Player (Variables|Default|GetPlayer1))))))))

(fn SetPlayerName
  (params (PlayerIndex :type Integer) (PlayerName :type String))
  (switch int PlayerIndex
    (:0
      (Variables|Default|SetPlayer0 (Utilities|Struct|MakeST_Player PlayerName (.Color (Utilities|Struct|BreakST_Player (Variables|Default|GetPlayer0))) (.Index (Utilities|Struct|BreakST_Player (Variables|Default|GetPlayer0))) (.isInCheckFlag (Utilities|Struct|BreakST_Player (Variables|Default|GetPlayer0))) (.HasLegalMoves (Utilities|Struct|BreakST_Player (Variables|Default|GetPlayer0))) (.MoveCount (Utilities|Struct|BreakST_Player (Variables|Default|GetPlayer0))) (.Captures (Utilities|Struct|BreakST_Player (Variables|Default|GetPlayer0))) (.currentChesscoins (Utilities|Struct|BreakST_Player (Variables|Default|GetPlayer0))))))
    (:1
      (Variables|Default|SetPlayer1 (Utilities|Struct|MakeST_Player PlayerName (.Color (Utilities|Struct|BreakST_Player (Variables|Default|GetPlayer1))) (.Index (Utilities|Struct|BreakST_Player (Variables|Default|GetPlayer1))) (.isInCheckFlag (Utilities|Struct|BreakST_Player (Variables|Default|GetPlayer1))) (.HasLegalMoves (Utilities|Struct|BreakST_Player (Variables|Default|GetPlayer1))) (.MoveCount (Utilities|Struct|BreakST_Player (Variables|Default|GetPlayer1))) (.Captures (Utilities|Struct|BreakST_Player (Variables|Default|GetPlayer1))) (.currentChesscoins (Utilities|Struct|BreakST_Player (Variables|Default|GetPlayer1))))))))

(fn IncrementPlayerMoveCount
  (params (PlayerIndex :type Integer))
  (switch int PlayerIndex
    (:0
      (Variables|Default|SetPlayer0 (Utilities|Struct|MakeST_Player (.Name (Utilities|Struct|BreakST_Player (Variables|Default|GetPlayer0))) (.Color (Utilities|Struct|BreakST_Player (Variables|Default|GetPlayer0))) (.Index (Utilities|Struct|BreakST_Player (Variables|Default|GetPlayer0))) (.isInCheckFlag (Utilities|Struct|BreakST_Player (Variables|Default|GetPlayer0))) (.HasLegalMoves (Utilities|Struct|BreakST_Player (Variables|Default|GetPlayer0))) (+ (.MoveCount (Utilities|Struct|BreakST_Player (Variables|Default|GetPlayer0))) 1) (.Captures (Utilities|Struct|BreakST_Player (Variables|Default|GetPlayer0))) (.currentChesscoins (Utilities|Struct|BreakST_Player (Variables|Default|GetPlayer0))))))
    (:1
      (Variables|Default|SetPlayer1 (Utilities|Struct|MakeST_Player (.Name (Utilities|Struct|BreakST_Player (Variables|Default|GetPlayer1))) (.Color (Utilities|Struct|BreakST_Player (Variables|Default|GetPlayer1))) (.Index (Utilities|Struct|BreakST_Player (Variables|Default|GetPlayer1))) (.isInCheckFlag (Utilities|Struct|BreakST_Player (Variables|Default|GetPlayer1))) (.HasLegalMoves (Utilities|Struct|BreakST_Player (Variables|Default|GetPlayer1))) (+ (.MoveCount (Utilities|Struct|BreakST_Player (Variables|Default|GetPlayer1))) 1) (.Captures (Utilities|Struct|BreakST_Player (Variables|Default|GetPlayer1))) (.currentChesscoins (Utilities|Struct|BreakST_Player (Variables|Default|GetPlayer1))))))))

(fn IncrementPlayerCaptureCount
  (params (PlayerIndex :type Integer))
  (switch int PlayerIndex
    (:0
      (Variables|Default|SetPlayer0 (Utilities|Struct|MakeST_Player (.Name (Utilities|Struct|BreakST_Player (Variables|Default|GetPlayer0))) (.Color (Utilities|Struct|BreakST_Player (Variables|Default|GetPlayer0))) (.Index (Utilities|Struct|BreakST_Player (Variables|Default|GetPlayer0))) (.isInCheckFlag (Utilities|Struct|BreakST_Player (Variables|Default|GetPlayer0))) (.HasLegalMoves (Utilities|Struct|BreakST_Player (Variables|Default|GetPlayer0))) (.MoveCount (Utilities|Struct|BreakST_Player (Variables|Default|GetPlayer0))) (+ (.Captures (Utilities|Struct|BreakST_Player (Variables|Default|GetPlayer0))) 1) (.currentChesscoins (Utilities|Struct|BreakST_Player (Variables|Default|GetPlayer0))))))
    (:1
      (Variables|Default|SetPlayer1 (Utilities|Struct|MakeST_Player (.Name (Utilities|Struct|BreakST_Player (Variables|Default|GetPlayer1))) (.Color (Utilities|Struct|BreakST_Player (Variables|Default|GetPlayer1))) (.Index (Utilities|Struct|BreakST_Player (Variables|Default|GetPlayer1))) (.isInCheckFlag (Utilities|Struct|BreakST_Player (Variables|Default|GetPlayer1))) (.HasLegalMoves (Utilities|Struct|BreakST_Player (Variables|Default|GetPlayer1))) (.MoveCount (Utilities|Struct|BreakST_Player (Variables|Default|GetPlayer1))) (+ (.Captures (Utilities|Struct|BreakST_Player (Variables|Default|GetPlayer1))) 1) (.currentChesscoins (Utilities|Struct|BreakST_Player (Variables|Default|GetPlayer1))))))))

(fn SetKinginCheckFlag
  (params (PlayerIndex :type Integer) (IsInCheck :type Boolean))
  (switch int PlayerIndex
    (:0
      (Variables|Default|SetPlayer0 (Utilities|Struct|MakeST_Player (.Name (Utilities|Struct|BreakST_Player (Variables|Default|GetPlayer0))) (.Color (Utilities|Struct|BreakST_Player (Variables|Default|GetPlayer0))) (.Index (Utilities|Struct|BreakST_Player (Variables|Default|GetPlayer0))) IsInCheck (.HasLegalMoves (Utilities|Struct|BreakST_Player (Variables|Default|GetPlayer0))) (.MoveCount (Utilities|Struct|BreakST_Player (Variables|Default|GetPlayer0))) (.Captures (Utilities|Struct|BreakST_Player (Variables|Default|GetPlayer0))) (.currentChesscoins (Utilities|Struct|BreakST_Player (Variables|Default|GetPlayer0))))))
    (:1
      (Variables|Default|SetPlayer1 (Utilities|Struct|MakeST_Player (.Name (Utilities|Struct|BreakST_Player (Variables|Default|GetPlayer1))) (.Color (Utilities|Struct|BreakST_Player (Variables|Default|GetPlayer1))) (.Index (Utilities|Struct|BreakST_Player (Variables|Default|GetPlayer1))) IsInCheck (.HasLegalMoves (Utilities|Struct|BreakST_Player (Variables|Default|GetPlayer1))) (.MoveCount (Utilities|Struct|BreakST_Player (Variables|Default|GetPlayer1))) (.Captures (Utilities|Struct|BreakST_Player (Variables|Default|GetPlayer1))) (.currentChesscoins (Utilities|Struct|BreakST_Player (Variables|Default|GetPlayer1))))))))

(fn SetHasLegalMovesFlag
  (params (PlayerIndex :type Integer) (HasLegalMoves :type Boolean))
  (switch int PlayerIndex
    (:0
      (Variables|Default|SetPlayer0 (Utilities|Struct|MakeST_Player (.Name (Utilities|Struct|BreakST_Player (Variables|Default|GetPlayer0))) (.Color (Utilities|Struct|BreakST_Player (Variables|Default|GetPlayer0))) (.Index (Utilities|Struct|BreakST_Player (Variables|Default|GetPlayer0))) (.isInCheckFlag (Utilities|Struct|BreakST_Player (Variables|Default|GetPlayer0))) HasLegalMoves (.MoveCount (Utilities|Struct|BreakST_Player (Variables|Default|GetPlayer0))) (.Captures (Utilities|Struct|BreakST_Player (Variables|Default|GetPlayer0))) (.currentChesscoins (Utilities|Struct|BreakST_Player (Variables|Default|GetPlayer0))))))
    (:1
      (Variables|Default|SetPlayer1 (Utilities|Struct|MakeST_Player (.Name (Utilities|Struct|BreakST_Player (Variables|Default|GetPlayer1))) (.Color (Utilities|Struct|BreakST_Player (Variables|Default|GetPlayer1))) (.Index (Utilities|Struct|BreakST_Player (Variables|Default|GetPlayer1))) (.isInCheckFlag (Utilities|Struct|BreakST_Player (Variables|Default|GetPlayer1))) HasLegalMoves (.MoveCount (Utilities|Struct|BreakST_Player (Variables|Default|GetPlayer1))) (.Captures (Utilities|Struct|BreakST_Player (Variables|Default|GetPlayer1))) (.currentChesscoins (Utilities|Struct|BreakST_Player (Variables|Default|GetPlayer1))))))))

(fn RotateCamera
  (params (Axis :type Float%20%28double-precision%29))
  (if (!= Axis 0.0)
    (Transformation|SetRelativeRotation (Variables|Default|GetCameraAzimuth) (Math|Rotator|MakeRotator 0.0 0.0 (+ Axis (.yaw (Variables|/Script/Engine.SceneComponent|GetRelativeRotation (Variables|Default|GetCameraAzimuth))))) false false)))

(fn SetPlayerChesscoins
  (params (PlayerIndex :type Integer) (PlayerChesscoins :type Integer))
  (switch int PlayerIndex
    (:0
      (Variables|Default|SetPlayer0 (Utilities|Struct|MakeST_Player (.Name (Utilities|Struct|BreakST_Player (Variables|Default|GetPlayer0))) (.Color (Utilities|Struct|BreakST_Player (Variables|Default|GetPlayer0))) (.Index (Utilities|Struct|BreakST_Player (Variables|Default|GetPlayer0))) (.isInCheckFlag (Utilities|Struct|BreakST_Player (Variables|Default|GetPlayer0))) (.HasLegalMoves (Utilities|Struct|BreakST_Player (Variables|Default|GetPlayer0))) (.MoveCount (Utilities|Struct|BreakST_Player (Variables|Default|GetPlayer0))) (.Captures (Utilities|Struct|BreakST_Player (Variables|Default|GetPlayer0))) PlayerChesscoins)))
    (:1
      (Variables|Default|SetPlayer1 (Utilities|Struct|MakeST_Player (.Name (Utilities|Struct|BreakST_Player (Variables|Default|GetPlayer1))) (.Color (Utilities|Struct|BreakST_Player (Variables|Default|GetPlayer1))) (.Index (Utilities|Struct|BreakST_Player (Variables|Default|GetPlayer1))) (.isInCheckFlag (Utilities|Struct|BreakST_Player (Variables|Default|GetPlayer1))) (.HasLegalMoves (Utilities|Struct|BreakST_Player (Variables|Default|GetPlayer1))) (.MoveCount (Utilities|Struct|BreakST_Player (Variables|Default|GetPlayer1))) (.Captures (Utilities|Struct|BreakST_Player (Variables|Default|GetPlayer1))) PlayerChesscoins)))))

(fn GetCurrentChesscoin
  (params (PlayerIndex :type Integer))
  (switch int PlayerIndex
    (:0
      (return (.currentChesscoins (Utilities|Struct|BreakST_Player (Variables|Default|GetPlayer0)))))
    (:1
      (return (.currentChesscoins (Utilities|Struct|BreakST_Player (Variables|Default|GetPlayer1)))))))

(fn SetBoughtFigures
  (params (PlayerIndex :type Integer))
  (switch int PlayerIndex
    (:0
      (Variables|Default|SetPlayer0 (Utilities|Struct|MakeST_Player "" (.Color (Utilities|Struct|BreakST_Player (Variables|Default|GetPlayer0))) (.Index (Utilities|Struct|BreakST_Player (Variables|Default|GetPlayer0))) (.isInCheckFlag (Utilities|Struct|BreakST_Player (Variables|Default|GetPlayer0))) (.HasLegalMoves (Utilities|Struct|BreakST_Player (Variables|Default|GetPlayer0))) (.MoveCount (Utilities|Struct|BreakST_Player (Variables|Default|GetPlayer0))) (.Captures (Utilities|Struct|BreakST_Player (Variables|Default|GetPlayer0))) (.currentChesscoins (Utilities|Struct|BreakST_Player (Variables|Default|GetPlayer0))) (+ (.BoughtFigures (Utilities|Struct|BreakST_Player (Variables|Default|GetPlayer0))) 1))))
    (:1
      (Variables|Default|SetPlayer1 (Utilities|Struct|MakeST_Player "" (.Color (Utilities|Struct|BreakST_Player (Variables|Default|GetPlayer1))) (.Index (Utilities|Struct|BreakST_Player (Variables|Default|GetPlayer1))) (.isInCheckFlag (Utilities|Struct|BreakST_Player (Variables|Default|GetPlayer1))) (.HasLegalMoves (Utilities|Struct|BreakST_Player (Variables|Default|GetPlayer1))) (.MoveCount (Utilities|Struct|BreakST_Player (Variables|Default|GetPlayer1))) (.Captures (Utilities|Struct|BreakST_Player (Variables|Default|GetPlayer1))) (.currentChesscoins (Utilities|Struct|BreakST_Player (Variables|Default|GetPlayer1))) (+ (.BoughtFigures (Utilities|Struct|BreakST_Player (Variables|Default|GetPlayer1))) 1))))))

(fn GetBoughtFigures
  (params (PlayerIndex :type Integer))
  (switch int PlayerIndex
    (:0
      (return (.BoughtFigures (Utilities|Struct|BreakST_Player (Variables|Default|GetPlayer0)))))
    (:1
      (return (.currentChesscoins (Utilities|Struct|BreakST_Player (Variables|Default|GetPlayer1)))))))